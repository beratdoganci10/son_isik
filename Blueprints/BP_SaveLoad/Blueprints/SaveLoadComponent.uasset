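; Component that saves and restores its owning object's data through the Resident Horror game instance, using world location as the object's key.
; On BeginPlay it caches its location, gets the game instance via a message call, and looks up stored data in ObjectSaveData.
; It then calls LoadedData with the result, or NoLoadedData if none exists.
; SaveData writes under the initial location, keeping the key stable if the object moves.
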(event `self.ReceiveBeginPlay`
  (set `self.Init Location` (`self.K2_GetComponentLocation`))
  (`self.Init Game Instance`)
  (`self.Loade Data`))

(fn `Init Game Instance`
  (bind _retrievergameinstanceresidenthorror (message `/Game/Son_Işık/Blueprints/BP_SaveLoad/Blueprints/BPI_SavemResidentHorror.RetrieverGameInstanceResidentHorror` (`GameplayStatics.GetGameInstance`)))
  (set `self.Game Instance Resident HorrorV1` _retrievergameinstanceresidenthorror))

(fn `Loade Data`
  (bind (_value _returnvalue) (`BlueprintMapLibrary.Map_Find` (`/Game/Son_Işık/Blueprints/BP_Core/ResidentHorrorV1_GameInstance.ObjectSaveData` (`self.Game Instance Resident HorrorV1`)) (`self.K2_GetComponentLocation`)))
  (if _returnvalue
    (bind _output_get (set `self.ST Stored data` _value))
    (`self.Loaded Data` _output_get)
    (else
      (`self.No loaded Data`))))

(fn `Save Data`
  (params (`Object Data` :type "/Game/Son_Işık/Blueprints/BP_SaveLoad/Structure/S_SaveLoad Structure"))
  (`/Game/Son_Işık/Blueprints/BP_Core/ResidentHorrorV1_GameInstance.SaveObjectData` (`self.Game Instance Resident HorrorV1`) `Object Data` (`self.Init Location`)))