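; Base interactable storage container that holds items and opens alongside the player's inventory with a sound.
; The construction script passes name, slot count and height to its inventory component.
; On BeginPlay it spawns zero-scale actors from the ContainerItems class-to-count map to copy their item structures into that inventory.
; Its save component records destruction and destroys it again on load; GetStoredInventory is an empty stub.
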(event `/Game/Son_Işık/Blueprints/BP_Interact/BPI_Interact.Interact Item`
  (params (ACTO :type "Actor Object Reference") (Player :type "/Game/Son_Işık/Character/BP_Character/BP_Resident_HorrorV1 Object Reference"))
  (bind _asbp_player (`/Game/Son_Işık/Blueprints/BP_FunctionLibray/BPFL_LibrayCharacter.My character Resident Horror`))
  (bind _bpc_inventory (`/Game/Son_Işık/Character/BP_Character/BP_Resident_HorrorV1.BPC_Inventory` _asbp_player))
  ; Start Interact
  (`/Game/Son_Işık/Blueprints/WBP/WBP_Player/WBP_HudPlayer.Additional elements  Visibility` (`/Game/Son_Işık/Character/BP_Character/BP_Resident_HorrorV1.WB HudPlayer` _asbp_player))
  (set `/Game/Son_Işık/Blueprints/BP_Inventory/BPC_Inventory.Container` self _bpc_inventory)
  (`self.GetStoredInventory`)
  (`/Game/Son_Işık/Blueprints/BP_Inventory/BPC_Inventory.Open/Close Inventory` _bpc_inventory)
  (`/Game/Son_Işık/Blueprints/BP_Inventory/BPC_Inventory.Open/Close Inventory` (`self.BPC_InventoryContainer`))
  (`GameplayStatics.PlaySound2D` "/Game/Son_Işık/Audio/WavFiles/WAV_inventory_opening_so__1-1768142816495.WAV_inventory_opening_so__1-1768142816495" 1.0 1.0 0.0 null null)
  (set `self.Open Inventory Container?` true))

(event `self.ReceiveBeginPlay`
  ; Not Remove
  (`parent.ReceiveBeginPlay`)
  (`self.PrepareContainer`))

(event `self.ReceiveDestroyed`
  (`/Game/Son_Işık/Blueprints/BP_SaveLoad/Blueprints/SaveLoadComponent.Save Data` (`self.SaveLoadComponent1`) (make `/Game/Son_Işık/Blueprints/BP_SaveLoad/Structure/S_SaveLoad` :`Boolean 1` true :`Music Manager` null :`Audio Component` null)))

(event `self.SaveLoadComponent1.Loaded Data`
  (params (`Save Loaded Data` :type "/Game/Son_Işık/Blueprints/BP_SaveLoad/Structure/S_SaveLoad Structure"))
  (if (`.Boolean1_7_53C431BB4280E2CC016B7F9971EC8093` (break `/Game/Son_Işık/Blueprints/BP_SaveLoad/Structure/S_SaveLoad` `Save Loaded Data`))
    (`self.K2_DestroyActor`)))

(fn `GetStoredInventory`)

(fn `PrepareContainer`
  (bind _values (`BlueprintMapLibrary.Map_Values` (`self.Container Items`)))
  (for (_array_element _array_index) _values
    (for _ (range _array_element)
      (bind _keys (`BlueprintMapLibrary.Map_Keys` (`self.Container Items`)))
      (bind _returnvalue (`|SpawnActorFromClass` (`|GetArrayItem` _keys _array_index) (`KismetMathLibrary.MakeTransform` (0.0 0.0 0.0) (struct) (0.0 0.0 0.0)) "Undefined" "MultiplyWithRoot" null null))
      (`/Game/Son_Işık/Blueprints/BP_Inventory/BPC_Inventory.Add To Inventory` (`self.BPC_InventoryContainer`) (make `/Game/Son_Işık/Blueprints/BP_Inventory/S_SlotStruct` (`.ItemStructure_3_D962DD8B4106829899F7C99F3F34F837` (break `/Game/Son_Işık/Blueprints/BP_Inventory/S_SlotStruct` (`/Game/Son_Işık/Blueprints/BP_Interact/BP_Master_Interact/BP_Master_Interact.S ItemStrucuture` _returnvalue))) 1)))))

(fn `UserConstructionScript`
  (bind _bpc_inventorycontainer (`self.BPC_InventoryContainer`))
  (set `/Game/Son_Işık/Blueprints/BP_Inventory/BPC_Inventory.Name` (`self.Name Storage`) _bpc_inventorycontainer)
  (set `/Game/Son_Işık/Blueprints/BP_Inventory/BPC_Inventory.NumberOfSlots` (`self.Container Slots`) _bpc_inventorycontainer)
  (set `/Game/Son_Işık/Blueprints/BP_Inventory/BPC_Inventory.InventoryHeight` (`self.Inventory Height`) _bpc_inventorycontainer)
  (`parent.UserConstructionScript`))