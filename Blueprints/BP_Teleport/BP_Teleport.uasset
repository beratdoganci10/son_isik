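; BP_Teleport is a trigger volume that moves the Resident Horror player character to a configured destination when that character overlaps its box.
; It disables input, fades the camera out, teleports the character, sets the controller's rotation to the destination rotation, then fades in and restores input.
; A parallel sequence branch plays timed fade sounds.
; The construction script writes the destination label to a text render.
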(event `self.Box.OnComponentBeginOverlap`
  (params (OverlappedComponent :type "PrimitiveComponent Object Reference") (OtherActor :type "Actor Object Reference") (OtherComp :type "PrimitiveComponent Object Reference") (OtherBodyIndex :type Integer) (bFromSweep :type Boolean) (SweepResult :type "HitResult Structure (by ref)"))
  (bind _asbp_player (`/Game/Son_Işık/Blueprints/BP_FunctionLibray/BPFL_LibrayCharacter.My character Resident Horror`))
  ;[0 0 0 0.5] Teleport
  (if (== OtherActor (`/Game/Son_Işık/Blueprints/BP_FunctionLibray/BPFL_LibrayCharacter.My character Resident Horror`))
    (`|ExecutionSequence`
      (:`then_0`
        (`self.DisableInput` self (`GameplayStatics.GetPlayerController` 0))
        (`PlayerCameraManager.StartCameraFade` :`self` (`GameplayStatics.GetPlayerCameraManager` 0) :`ToAlpha` 1.0 :`Duration` 1.0)
        (`KismetSystemLibrary.Delay` 1.0)
        (`self.K2_TeleportTo` :`self` _asbp_player :`DestLocation` (`self.Dest Location`))
        (`Controller.SetControlRotation` (`Pawn.GetController` _asbp_player) (`self.Dest Rotation`))
        (`PlayerCameraManager.StartCameraFade` :`self` (`GameplayStatics.GetPlayerCameraManager` 0) :`FromAlpha` 2.0 :`Duration` 1.0)
        (`self.EnableInput` self (`GameplayStatics.GetPlayerController` 0)))
      (:`then_1`
        (`KismetSystemLibrary.Delay` 0.2)
        (`GameplayStatics.PlaySound2D` "/Game/Son_Işık/Audio/WavFiles/WAV_ShotFadIn.WAV_ShotFadIn" 1.0 1.0 0.0 null null)
        (`KismetSystemLibrary.Delay` 1.4)
        (`GameplayStatics.PlaySound2D` "/Engine/VREditor/Sounds/UI/Radial_Menu_FadeOut.Radial_Menu_FadeOut" 3.0 1.0 0.0 null null)))))

(fn `UserConstructionScript`
  (`TextRenderComponent.K2_SetText` (`self.TextRender`) (`self.Write destination`)))