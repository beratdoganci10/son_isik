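; Weapon component that handles firing, reloading and laser attachments for the player character's equipped weapon.
; A looping timer repeats shots at the weapon's firing rate, checking ammo and line-tracing once, or per pellet for shotguns.
; Shots spawn projectiles, apply damage through BPI_DamageWeapon, trigger recoil and feedback, and place decals with surface-specific impact effects.
; Reload refills the clip from inventory ammo, and laser functions spawn or hide a socket-attached BP_Laser.
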(event `Start Shooting`
  (bind _asbp_player (`/Game/Son_Işık/Blueprints/BP_FunctionLibray/BPFL_LibrayCharacter.My character Resident Horror`))
  (bind _asbp_player_2 (`/Game/Son_Işık/Blueprints/BP_FunctionLibray/BPFL_LibrayCharacter.My character Resident Horror`))
  (bind _asbp_player_3 (`/Game/Son_Işık/Blueprints/BP_FunctionLibray/BPFL_LibrayCharacter.My character Resident Horror`))
  (bind (_returnvalue _returnvalue1) (`/Game/Son_Işık/Character/BP_Character/BP_Resident_HorrorV1.Line Trace Weapon` _asbp_player_3))
  (bind _equipped_weapon (`/Game/Son_Işık/Character/BP_Character/BP_Resident_HorrorV1.Equipped Weapon` (`/Game/Son_Işık/Blueprints/BP_FunctionLibray/BPFL_LibrayCharacter.My character Resident Horror`)))
  (bind _equipped_weapon_2 (`/Game/Son_Işık/Character/BP_Character/BP_Resident_HorrorV1.Equipped Weapon` (`/Game/Son_Işık/Blueprints/BP_FunctionLibray/BPFL_LibrayCharacter.My character Resident Horror`)))
  (bind _equipped_weapon_3 (`/Game/Son_Işık/Character/BP_Character/BP_Resident_HorrorV1.Equipped Weapon` _asbp_player_2))
  (bind _equipped_weapon_4 (`/Game/Son_Işık/Character/BP_Character/BP_Resident_HorrorV1.Equipped Weapon` (`/Game/Son_Işık/Blueprints/BP_FunctionLibray/BPFL_LibrayCharacter.My character Resident Horror`)))
  (bind _returnvalue_2 (`KismetMathLibrary.GetForwardVector` _returnvalue1))
  ;[0 0 0 1 42] Shooting Weapon
  (set `self.is shooting?` true)
  (bind _returnvalue_3 (`KismetSystemLibrary.K2_SetTimerDelegate` (delegate `Fire Rate`) (`/Game/Son_Işık/Blueprints/BP_Weapon/BP_BaseWeapon/BP_Base_Weapon.Firing Rate` (`/Game/Son_Işık/Character/BP_Character/BP_Resident_HorrorV1.Equipped Weapon` (`/Game/Son_Işık/Blueprints/BP_FunctionLibray/BPFL_LibrayCharacter.My character Resident Horror`))) true))
  (set `self.Fire Rate Weapon` _returnvalue_3)
  (`/Engine/EditorBlueprintResources/StandardMacros.IsValid` (`/Game/Son_Işık/Character/BP_Character/BP_Resident_HorrorV1.Equipped Weapon` (`/Game/Son_Işık/Blueprints/BP_FunctionLibray/BPFL_LibrayCharacter.My character Resident Horror`)) :!label _label
    (:`Is Valid`
      (`|ExecutionSequence`
        (:`then_0`
          (goto _label_2 :!via `Open`))
        (:`then_1`
          (`/Engine/EditorBlueprintResources/StandardMacros.Gate` true :!label _label_2
            (:`Exit`
              (if (<= (`/Game/Son_Işık/Blueprints/BP_Weapon/BP_BaseWeapon/BP_Base_Weapon.Current Ammo` (`/Game/Son_Işık/Character/BP_Character/BP_Resident_HorrorV1.Equipped Weapon` (`/Game/Son_Işık/Blueprints/BP_FunctionLibray/BPFL_LibrayCharacter.My character Resident Horror`))) 0)
                (`GameplayStatics.PlaySound2D` "/Game/Son_Işık/Audio/UI/WAV_Hovered.WAV_Hovered" 1.0 1.0 0.0 null null)
                (else
                  (`GameplayStatics.SpawnSoundAtLocation` (`/Game/Son_Işık/Blueprints/BP_Weapon/BP_BaseWeapon/BP_Base_Weapon.Sound Shooting` (`/Game/Son_Işık/Character/BP_Character/BP_Resident_HorrorV1.Equipped Weapon` _asbp_player)) (`Actor.K2_GetActorLocation` _asbp_player) (`Actor.K2_GetActorRotation` _asbp_player) 1.0 1.0 0.0 null null)
                  (if (`/Game/Son_Işık/Blueprints/BP_Weapon/BP_BaseWeapon/BP_Base_Weapon.Fire Shotgun?` (`/Game/Son_Işık/Character/BP_Character/BP_Resident_HorrorV1.Equipped Weapon` (`/Game/Son_Işık/Blueprints/BP_FunctionLibray/BPFL_LibrayCharacter.My character Resident Horror`)))
                    (`KismetArrayLibrary.Array_Clear` (`self.touched surfaces`))
                    (for _ (range 1 (+ (`/Game/Son_Işık/Blueprints/BP_Weapon/BP_BaseWeapon/BP_Base_Weapon.Quanty Shot Shotgun?` _equipped_weapon_2) 1))
                      (bind (_outhit _returnvalue_4) (`KismetSystemLibrary.LineTraceSingle` :`Start` _returnvalue :`End` (+ (+ _returnvalue (* _returnvalue_2 (`/Game/Son_Işık/Blueprints/BP_Weapon/BP_BaseWeapon/BP_Base_Weapon.Shooting Range` (`/Game/Son_Işık/Character/BP_Character/BP_Resident_HorrorV1.Equipped Weapon` _asbp_player_3)))) (`KismetMathLibrary.MakeVector` (`KismetMathLibrary.RandomFloatInRange` 0.0 (`/Game/Son_Işık/Blueprints/BP_Weapon/BP_BaseWeapon/BP_Base_Weapon.Echo X Bullet Spread` _equipped_weapon_2)) (`KismetMathLibrary.RandomFloatInRange` 0.0 (`/Game/Son_Işık/Blueprints/BP_Weapon/BP_BaseWeapon/BP_Base_Weapon.Echo Y Bullet Spreader` _equipped_weapon_2)) (`KismetMathLibrary.RandomFloatInRange` 0.0 (`/Game/Son_Işık/Blueprints/BP_Weapon/BP_BaseWeapon/BP_Base_Weapon.Spread Echo Z candy` _equipped_weapon_2)))) :`TraceChannel` "TraceTypeQuery4" :`DrawDebugType` (select `bool` (`/Game/Son_Işık/Blueprints/BP_Weapon/BP_BaseWeapon/BP_Base_Weapon.Debug Line Trace?` (`/Game/Son_Işık/Character/BP_Character/BP_Resident_HorrorV1.Equipped Weapon` (`/Game/Son_Işık/Blueprints/BP_FunctionLibray/BPFL_LibrayCharacter.My character Resident Horror`))) :`true` "ForDuration" :!type "EDrawDebugTrace Enum") :`DrawTime` 1.0 :!label _label_3))
                      (if _returnvalue_4
                        (bind (_bblockinghit _binitialoverlap _time _distance _location _impactpoint _normal _impactnormal _physmat _hitactor _hitcomponent _hitbonename _bonename _hititem _elementindex _faceindex _tracestart _traceend) (`GameplayStatics.BreakHitResult` _outhit))
                        (`self.Effect Weapon` _impactpoint (select `bool` _returnvalue_4 :`false` _traceend :`true` _impactpoint) _returnvalue_4 _normal _location (`PhysicalMaterial.SurfaceType` _physmat) _hitcomponent))
                      (`|SpawnActorFromClass` "/Game/Son_Işık/Blueprints/BP_Weapon/BP_BaseWeapon/BP_ProjectTile/BP_Projecttile.BP_Projecttile_C" (`KismetMathLibrary.MakeTransform` _returnvalue (`KismetMathLibrary.Conv_VectorToRotator` _returnvalue_2)) "Undefined" "MultiplyWithRoot" null null)
                      (`self.Apply Damage Weapon` _hitactor _outhit)
                      (`/Game/Son_Işık/Blueprints/BP_Weapon/BP_BaseWeapon/BP_Base_Weapon.Animation Shooting` _equipped_weapon)
                      (`/Game/Son_Işık/Blueprints/BP_Weapon/BP_BaseWeapon/BP_Base_Weapon.Animation Weapon Shooting` _equipped_weapon)
                      (`GameplayStatics.SpawnEmitterAttached` "/Game/Son_Işık/ParticleEffects/PS_AssaultRifle_MuzzleFlash.PS_AssaultRifle_MuzzleFlash" (`/Game/Son_Işık/Blueprints/BP_Interact/BP_Master_Interact/BP_Master_Interact.SkeletalMesh` _equipped_weapon) "Muzzle" (0.0 0.0 0.0) (struct) (1.0 1.0 1.0) "SnapToTarget")
                      (`/Game/Son_Işık/Blueprints/BP_Weapon/BP_BaseWeapon/BP_Base_Weapon.Recoil Weapon` _equipped_weapon_3 _asbp_player_2)
                      (`GameplayStatics.PlayWorldCameraShake` (`/Game/Son_Işık/Blueprints/BP_Weapon/BP_BaseWeapon/BP_Base_Weapon.Camera Shake` _equipped_weapon_3) (`SceneComponent.K2_GetComponentLocation` (`/Game/Son_Işık/Character/BP_Character/BP_Resident_HorrorV1.Camera` _asbp_player_2)) 600.0 600.0)
                      (if (not (`/Game/Son_Işık/Blueprints/BP_Weapon/BP_BaseWeapon/BP_Base_Weapon.Fire Shotgun?` _equipped_weapon_4))
                        (`/Game/Son_Işık/Blueprints/BP_Weapon/BP_BaseWeapon/BP_Base_Weapon.Cassing` _equipped_weapon_4 (`/Game/Son_Işık/Blueprints/BP_Interact/BP_Master_Interact/BP_Master_Interact.SkeletalMesh` _equipped_weapon_4))))
                    (`self.Decrease Ammo`)
                    (else
                      (`self.Decrease Ammo`)
                      (goto _label_3))))))))))))

(event `Fire Rate`
  ;[0 0 0 1 42] Shooting Weapon
  (if (`self.is shooting?`)
    (goto _label)))

(event `Stop Shooting`
  ;[0 0 0 1 42] Shooting Weapon
  (`KismetSystemLibrary.K2_ClearAndInvalidateTimerHandle` (`self.Fire Rate Weapon`))
  (goto _label_2 :!via `Close`))

(event `Reload Weapon`
  (bind _equipped_weapon (`/Game/Son_Işık/Character/BP_Character/BP_Resident_HorrorV1.Equipped Weapon` (`/Game/Son_Işık/Blueprints/BP_FunctionLibray/BPFL_LibrayCharacter.My character Resident Horror`)))
  ;[0 0 0 1 45] Reload Weapon
  (`/Engine/EditorBlueprintResources/StandardMacros.IsValid` (`/Game/Son_Işık/Character/BP_Character/BP_Resident_HorrorV1.Equipped Weapon` (`/Game/Son_Işık/Blueprints/BP_FunctionLibray/BPFL_LibrayCharacter.My character Resident Horror`))
    (:`Is Valid`
      (if (and (> (`self.Get Ammo on inventory`) 0) (!= (`/Game/Son_Işık/Blueprints/BP_Weapon/BP_BaseWeapon/BP_Base_Weapon.Default Ammo on Clip` _equipped_weapon) (`/Game/Son_Işık/Blueprints/BP_Weapon/BP_BaseWeapon/BP_Base_Weapon.Current Ammo` _equipped_weapon)))
        (`self.Set reloaded ammo`)
        (`self.Applying Recharge Animation`)))))

(event `Applying Recharge Animation`
  ;[0 0 0 1 45] Reload Weapon
  ;;[1 0.8719 0.8719 0.5] Applying Recharge Animation
  (`/Game/Son_Işık/Blueprints/BP_Weapon/BP_BaseWeapon/BP_Base_Weapon.Animation Reload Weapon` (`/Game/Son_Işık/Character/BP_Character/BP_Resident_HorrorV1.Equipped Weapon` (`/Game/Son_Işık/Blueprints/BP_FunctionLibray/BPFL_LibrayCharacter.My character Resident Horror`))))

(fn `Activae Laser`
  (bind _equipped_weapon (`/Game/Son_Işık/Character/BP_Character/BP_Resident_HorrorV1.Equipped Weapon` (`/Game/Son_Işık/Blueprints/BP_FunctionLibray/BPFL_LibrayCharacter.My character Resident Horror`)))
  (`/Engine/EditorBlueprintResources/StandardMacros.IsValid` _equipped_weapon
    (:`Is Valid`
      (if (`/Game/Son_Işık/Blueprints/BP_Weapon/BP_BaseWeapon/BP_Base_Weapon.Have laser?` _equipped_weapon)
        (bind _returnvalue (`|SpawnActorFromClass` "/Game/Son_Işık/Blueprints/Bp_Laser/BP_Laser.BP_Laser_C" (`SceneComponent.GetSocketTransform` (`/Game/Son_Işık/Blueprints/BP_Interact/BP_Master_Interact/BP_Master_Interact.SkeletalMesh` _equipped_weapon) "Laser" "RTS_World") "Undefined" "MultiplyWithRoot" null null))
        (bind _output_get (set `self.BP Laser` _returnvalue))
        (bind _laserequipament (`/Game/Son_Işık/Blueprints/Bp_Laser/BP_Laser.LaserEquipament` _output_get))
        (`SceneComponent.K2_AttachToComponent` _laserequipament (`/Game/Son_Işık/Blueprints/BP_Interact/BP_Master_Interact/BP_Master_Interact.SkeletalMesh` (`/Game/Son_Işık/Character/BP_Character/BP_Resident_HorrorV1.Equipped Weapon` (`/Game/Son_Işık/Blueprints/BP_FunctionLibray/BPFL_LibrayCharacter.My character Resident Horror`))) "Laser" "SnapToTarget" "SnapToTarget" "KeepWorld" true)
        (`StaticMeshComponent.SetStaticMesh` _laserequipament (`/Game/Son_Işık/Blueprints/BP_Inventory/DA_BaseInteract.Mesh Laser Equipament` (`.DA_BaseInteract_112_E5D63A474E86D51C38EA9ABF9499DC91` (break `/Game/Son_Işık/Blueprints/BP_Inventory/S_Item_Structure` (`.ItemStructure_3_D962DD8B4106829899F7C99F3F34F837` (break `/Game/Son_Işık/Blueprints/BP_Inventory/S_SlotStruct` (`/Game/Son_Işık/Blueprints/BP_Interact/BP_Master_Interact/BP_Master_Interact.S ItemStrucuture` (`/Game/Son_Işık/Character/BP_Character/BP_Resident_HorrorV1.Equipped Weapon` (`/Game/Son_Işık/Blueprints/BP_FunctionLibray/BPFL_LibrayCharacter.My character Resident Horror`)))))))))))))

(fn `Apply Damage Weapon`
  (params (Acto :type "Actor Object Reference") (HitResult :type "HitResult Structure"))
  (if (`KismetSystemLibrary.DoesImplementInterface` Acto "/Game/Son_Işık/Blueprints/BP_Weapon/BP_BaseWeapon/Structure/BPI_DamageWeapon.BPI_DamageWeapon_C")
    (message `/Game/Son_Işık/Blueprints/BP_Weapon/BP_BaseWeapon/Structure/BPI_DamageWeapon.Event Damage` Acto (`/Game/Son_Işık/Blueprints/BP_Inventory/DA_BaseInteract.Damage` (`.DA_BaseInteract_112_E5D63A474E86D51C38EA9ABF9499DC91` (break `/Game/Son_Işık/Blueprints/BP_Inventory/S_Item_Structure` (`.ItemStructure_3_D962DD8B4106829899F7C99F3F34F837` (break `/Game/Son_Işık/Blueprints/BP_Inventory/S_SlotStruct` (`/Game/Son_Işık/Blueprints/BP_Interact/BP_Master_Interact/BP_Master_Interact.S ItemStrucuture` (`/Game/Son_Işık/Character/BP_Character/BP_Resident_HorrorV1.Equipped Weapon` (`/Game/Son_Işık/Blueprints/BP_FunctionLibray/BPFL_LibrayCharacter.My character Resident Horror`)))))))) HitResult)))

(fn `Deactivate Laser`
  (bind _equipped_weapon (`/Game/Son_Işık/Character/BP_Character/BP_Resident_HorrorV1.Equipped Weapon` (`/Game/Son_Işık/Blueprints/BP_FunctionLibray/BPFL_LibrayCharacter.My character Resident Horror`)))
  (`/Engine/EditorBlueprintResources/StandardMacros.IsValid` _equipped_weapon
    (:`Is Valid`
      (if (`/Game/Son_Işık/Blueprints/BP_Weapon/BP_BaseWeapon/BP_Base_Weapon.Have laser?` _equipped_weapon)
        (`Actor.SetActorHiddenInGame` (`self.BP Laser`) true)))))

(fn `Decrease Ammo`
  (`/Game/Son_Işık/Blueprints/BP_Weapon/BP_BaseWeapon/BP_Base_Weapon.Decrease Ammo` (`/Game/Son_Işık/Character/BP_Character/BP_Resident_HorrorV1.Equipped Weapon` (`/Game/Son_Işık/Blueprints/BP_FunctionLibray/BPFL_LibrayCharacter.My character Resident Horror`))))

(fn `Effect Weapon`
  (params (`Start point` :type "Vector Structure") (EndPOint :type "Vector Structure") (`Does Hit` :type Boolean) (Normal :type "Vector Structure") (Location :type "Vector Structure") (SurfaceType :type "EPhysicalSurface Enum" :default "SurfaceType_Default") (AttachToComponent :type "SceneComponent Object Reference"))
  (bind (_returnvalue_roll _returnvalue_pitch) (`KismetMathLibrary.BreakRotator` (`KismetMathLibrary.RandomRotator` false)))
  (bind _returnvalue (`KismetMathLibrary.Conv_VectorToRotator` Normal))
  (bind _returnvalue_2 (`KismetMathLibrary.NormalizedDeltaRotator` _returnvalue (`KismetMathLibrary.MakeRotator` 0.0 _returnvalue_pitch)))
  (bind _da_baseinteract (break `/Game/Son_Işık/Blueprints/BP_Inventory/S_Item_Structure` (`.ItemStructure_3_D962DD8B4106829899F7C99F3F34F837` (break `/Game/Son_Işık/Blueprints/BP_Inventory/S_SlotStruct` (`/Game/Son_Işık/Blueprints/BP_Interact/BP_Master_Interact/BP_Master_Interact.S ItemStrucuture` (`/Game/Son_Işık/Character/BP_Character/BP_Resident_HorrorV1.Equipped Weapon` (`/Game/Son_Işık/Blueprints/BP_FunctionLibray/BPFL_LibrayCharacter.My character Resident Horror`)))))))
  (if `Does Hit`
    (bind _returnvalue_3 (`GameplayStatics.SpawnDecalAttached` (`/Game/Son_Işık/Blueprints/BP_Inventory/DA_BaseInteract.Decal Impact Weapon` _da_baseinteract) (`/Game/Son_Işık/Blueprints/BP_Inventory/DA_BaseInteract.Decal Size` _da_baseinteract) AttachToComponent "None" Location _returnvalue "KeepWorldPosition" 10.0))
    (`DecalComponent.SetFadeScreenSize` _returnvalue_3 0.0001)
    (switch `EPhysicalSurface` SurfaceType
      (:`SurfaceType_Default`
        (`GameplayStatics.SpawnEmitterAtLocation` (`/Game/Son_Işık/Blueprints/BP_CustomDataAssets/Base/DA_Fx_Weapon.Impact Weapon Default ` (`self.Bp Impact Weapon`)) Location _returnvalue_2)
        (`GameplayStatics.PlaySoundAtLocation` (`/Game/Son_Işık/Blueprints/BP_CustomDataAssets/Base/DA_Sfx_Weapon.Sound Impact Weapon Default ` (`self.Bp Sound Impact Weapon`)) Location (struct) 1.0 1.0 0.0 "/Game/Son_Işık/Audio/Attenuation/SA_Door.SA_Door" null null null))
      (:`SurfaceType1`
        (`GameplayStatics.SpawnEmitterAtLocation` (`/Game/Son_Işık/Blueprints/BP_CustomDataAssets/Base/DA_Fx_Weapon.Impact Weapon Metal` (`self.Bp Impact Weapon`)) Location _returnvalue_2)
        (`GameplayStatics.PlaySoundAtLocation` (`/Game/Son_Işık/Blueprints/BP_CustomDataAssets/Base/DA_Sfx_Weapon.Sound Impact Weapon Metal` (`self.Bp Sound Impact Weapon`)) Location (struct) 2.0 1.0 0.0 "/Game/Son_Işık/Audio/Attenuation/SA_Door.SA_Door" null null null))
      (:`SurfaceType2`
        (`NiagaraFunctionLibrary.SpawnSystemAtLocation` (`/Game/Son_Işık/Blueprints/BP_CustomDataAssets/Base/DA_Fx_Weapon.Impact Weapon Water` (`self.Bp Impact Weapon`)) Location _returnvalue_2)
        (`GameplayStatics.PlaySoundAtLocation` (`/Game/Son_Işık/Blueprints/BP_CustomDataAssets/Base/DA_Sfx_Weapon.Sound Impact Weapon Water` (`self.Bp Sound Impact Weapon`)) Location (struct) 2.0 1.0 0.0 "/Game/Son_Işık/Audio/Attenuation/SA_Door.SA_Door" null null null))
      (:`SurfaceType3`
        (`GameplayStatics.SpawnEmitterAtLocation` (`/Game/Son_Işık/Blueprints/BP_CustomDataAssets/Base/DA_Fx_Weapon.Impact Weapon Concret` (`self.Bp Impact Weapon`)) Location _returnvalue_2)
        (`GameplayStatics.PlaySoundAtLocation` (`/Game/Son_Işık/Blueprints/BP_CustomDataAssets/Base/DA_Sfx_Weapon.Sound Impact Weapon Concret` (`self.Bp Sound Impact Weapon`)) Location (struct) 1.0 1.0 0.0 "/Game/Son_Işık/Audio/Attenuation/SA_Door.SA_Door" null null null))
      (:`SurfaceType4`
        (`NiagaraFunctionLibrary.SpawnSystemAtLocation` (`/Game/Son_Işık/Blueprints/BP_CustomDataAssets/Base/DA_Fx_Weapon.Impact Weapon Grass` (`self.Bp Impact Weapon`)) Location _returnvalue_2)
        (`GameplayStatics.PlaySoundAtLocation` (`/Game/Son_Işık/Blueprints/BP_CustomDataAssets/Base/DA_Sfx_Weapon.Sound Impact Weapon Grass` (`self.Bp Sound Impact Weapon`)) Location (struct) 2.0 1.0 0.0 "/Game/Son_Işık/Audio/Attenuation/SA_Door.SA_Door" null null null))
      (:`SurfaceType5`
        (`NiagaraFunctionLibrary.SpawnSystemAtLocation` (`/Game/Son_Işık/Blueprints/BP_CustomDataAssets/Base/DA_Fx_Weapon.Impact Weapon Blood` (`self.Bp Impact Weapon`)) Location _returnvalue_2)
        (`GameplayStatics.PlaySoundAtLocation` (`/Game/Son_Işık/Blueprints/BP_CustomDataAssets/Base/DA_Sfx_Weapon.Sound Impact Weapon Blood` (`self.Bp Sound Impact Weapon`)) Location (struct) 2.0 1.0 0.0 "/Game/Son_Işık/Audio/Attenuation/SA_Door.SA_Door" null null null))
      (:`SurfaceType6`
        (`GameplayStatics.SpawnEmitterAtLocation` (`/Game/Son_Işık/Blueprints/BP_CustomDataAssets/Base/DA_Fx_Weapon.Impact Weapon Wood` (`self.Bp Impact Weapon`)) Location _returnvalue_2)
        (`GameplayStatics.PlaySoundAtLocation` (`/Game/Son_Işık/Blueprints/BP_CustomDataAssets/Base/DA_Sfx_Weapon.Sound Impact Weapon Wood` (`self.Bp Sound Impact Weapon`)) Location (struct) 1.0 1.0 0.0 "/Game/Son_Işık/Audio/Attenuation/SA_Door.SA_Door" null null null))))
  (return))

(fn `Get Ammo on inventory`
  (returns (ReturnValue :type Integer))
  (bind _asbp_player (`/Game/Son_Işık/Blueprints/BP_FunctionLibray/BPFL_LibrayCharacter.My character Resident Horror`))
  (return (`/Game/Son_Işık/Blueprints/BP_Inventory/BPC_Inventory.Get Item quantity` (`/Game/Son_Işık/Character/BP_Character/BP_Resident_HorrorV1.BPC_Inventory` _asbp_player) (`/Game/Son_Işık/Blueprints/BP_Weapon/BP_BaseWeapon/BP_Base_Weapon.My ammo type` (`/Game/Son_Işık/Character/BP_Character/BP_Resident_HorrorV1.Equipped Weapon` _asbp_player)))))

(fn `Set reloaded ammo`
  (locals (`RECARGA MUNIÇÃO NECESSARIA` :type Integer) (`Leftover ammo on clip` :type Integer :default 0))
  (bind _asbp_player (`/Game/Son_Işık/Blueprints/BP_FunctionLibray/BPFL_LibrayCharacter.My character Resident Horror`))
  (bind _equipped_weapon (`/Game/Son_Işık/Character/BP_Character/BP_Resident_HorrorV1.Equipped Weapon` (`/Game/Son_Işık/Blueprints/BP_FunctionLibray/BPFL_LibrayCharacter.My character Resident Horror`)))
  (set `local.Leftover ammo on clip` (`/Game/Son_Işık/Blueprints/BP_Weapon/BP_BaseWeapon/BP_Base_Weapon.Current Ammo` (`/Game/Son_Işık/Character/BP_Character/BP_Resident_HorrorV1.Equipped Weapon` (`/Game/Son_Işık/Blueprints/BP_FunctionLibray/BPFL_LibrayCharacter.My character Resident Horror`))))
  (set `/Game/Son_Işık/Blueprints/BP_Weapon/BP_BaseWeapon/BP_Base_Weapon.Current Ammo` (`KismetMathLibrary.Clamp` (`/Game/Son_Işık/Blueprints/BP_Weapon/BP_BaseWeapon/BP_Base_Weapon.Default Ammo on Clip` (`/Game/Son_Işık/Character/BP_Character/BP_Resident_HorrorV1.Equipped Weapon` (`/Game/Son_Işık/Blueprints/BP_FunctionLibray/BPFL_LibrayCharacter.My character Resident Horror`))) 0 (+ (`self.Get Ammo on inventory`) (`local.Leftover ammo on clip`))) _equipped_weapon)
  (`/Game/Son_Işık/Blueprints/BP_Weapon/BP_BaseWeapon/BP_Base_Weapon.Update Ammo on game instance` _equipped_weapon)
  (`/Game/Son_Işık/Blueprints/BP_Inventory/BPC_Inventory.Remove From Inventory` (`/Game/Son_Işık/Character/BP_Character/BP_Resident_HorrorV1.BPC_Inventory` _asbp_player) (make `/Game/Son_Işık/Blueprints/BP_Inventory/S_SlotStruct` (make `/Game/Son_Işık/Blueprints/BP_Inventory/S_Item_Structure` (`/Game/Son_Işık/Blueprints/BP_Weapon/BP_BaseWeapon/BP_Base_Weapon.My ammo type` (`/Game/Son_Işık/Character/BP_Character/BP_Resident_HorrorV1.Equipped Weapon` _asbp_player))) (- (`/Game/Son_Işık/Blueprints/BP_Weapon/BP_BaseWeapon/BP_Base_Weapon.Default Ammo on Clip` (`/Game/Son_Işık/Character/BP_Character/BP_Resident_HorrorV1.Equipped Weapon` _asbp_player)) (`local.Leftover ammo on clip`)))))